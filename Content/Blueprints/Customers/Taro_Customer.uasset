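; Taro customer actor for a cooking game that walks in, sits, and leaves when interacted with.
; On BeginPlay a Timeline lerps it 550 units along Y with a walk animation, then switches to sitting.
; Interactwith turns the mesh, walks it back on a second Timeline, and shows Dialogue in the CookingManager's speech bubble.
; A Delay on that Timeline's Update hides the bubble and destroys the actor after three seconds.
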(event `self.ReceiveBeginPlay`
  (bind _returnvalue (`self.K2_GetActorLocation`))
  (bind _output_get (set `self.MoveStart` _returnvalue))
  (bind _output_get_2 (set `self.MovEnd` (+ _returnvalue (0.0 550.0 0.0))))
  (`SkeletalMeshComponent.PlayAnimation` (`self.Mesh`) "/Game/Characters/Animations/AN_Walk_Anim.AN_Walk_Anim" true)
  (bind (_direction _newtrack_1) (`Timeline|Timeline` :!via `PlayFromStart`)
    (:`Update`
      (`self.K2_SetActorLocation` (`KismetMathLibrary.VLerp` _output_get _output_get_2 _newtrack_1)))
    (:`Finished`
      (`SkeletalMeshComponent.PlayAnimation` (`self.Mesh`) "/Game/Characters/Animations/AN_Sit_Anim.AN_Sit_Anim" true))))

(event `self.Box.OnComponentBeginOverlap`
  (params (OverlappedComponent :type "PrimitiveComponent Object Reference") (OtherActor :type "Actor Object Reference") (OtherComp :type "PrimitiveComponent Object Reference") (OtherBodyIndex :type Integer) (bFromSweep :type Boolean) (SweepResult :type "HitResult Structure (by ref)")))

(event `/Game/Blueprints/KitchenStuff/I_InteractInterface.InteractWith`
  (params (CookingManager :type "/Game/Blueprints/KitchenStuff/BP_CookingManager Object Reference") (Ingredient :type "/Game/Blueprints/KitchenStuff/BP_Ingredient Object Reference"))
  (bind _returnvalue (`self.K2_GetActorLocation`))
  (bind _ui_widget (`self.UI Widget`))
  (set `self.UI Widget` (`/Game/Blueprints/KitchenStuff/BP_CookingManager.SpeechBubble` CookingManager))
  (bind _output_get (set `self.MoveStart` _returnvalue))
  (bind _output_get_2 (set `self.MovEnd` (+ _returnvalue (0.0 -550.0 0.0))))
  (`SkeletalMeshComponent.PlayAnimation` (`self.Mesh`) "/Game/Characters/Animations/AN_Walk_Anim.AN_Walk_Anim" true)
  (`SceneComponent.K2_SetRelativeRotation` (`self.Mesh`) (struct :`Yaw` 90.0) false false)
  (bind (_direction _newtrack_1) (`Timeline|Timeline_0` :!via `PlayFromStart`)
    (:`Update`
      (`self.K2_SetActorLocation` (`KismetMathLibrary.VLerp` _output_get _output_get_2 _newtrack_1))
      (`Widget.SetVisibility` _ui_widget "Visible")
      (`/Game/Blueprints/UI/SpeechBubble.UpdateText` _ui_widget (`self.Dialogue`))
      (`KismetSystemLibrary.Delay` 3.0)
      (`Widget.SetVisibility` _ui_widget "Hidden")
      (`self.K2_DestroyActor`))))

(fn `UserConstructionScript`)