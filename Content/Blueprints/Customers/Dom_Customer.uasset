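; Dom customer actor that walks in along Y on spawn, then loops a sit animation.
; When the player overlaps its box, it shows a hardcoded line in a Text widget, turns its mesh and walks back the opposite way.
; Both walks lerp location through timelines.
; The exit timeline's Update also starts a delay that clears the text and destroys the actor, timed from the walk's start rather than its finish.
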(event `self.ReceiveBeginPlay`
  (bind _returnvalue (`self.K2_GetActorLocation`))
  (bind _output_get (set `self.MoveStart` _returnvalue))
  (bind _output_get_2 (set `self.MovEnd` (+ _returnvalue (0.0 550.0 0.0))))
  (`SkeletalMeshComponent.PlayAnimation` (`self.Mesh`) "/Game/Characters/Animations/AN_Walk_Anim.AN_Walk_Anim" true)
  (bind (_direction _newtrack_1) (`Timeline|Timeline` :!via `PlayFromStart`)
    (:`Update`
      (`self.K2_SetActorLocation` (`KismetMathLibrary.VLerp` _output_get _output_get_2 _newtrack_1)))
    (:`Finished`
      (`SkeletalMeshComponent.PlayAnimation` (`self.Mesh`) "/Game/Characters/Animations/AN_Sit_Anim.AN_Sit_Anim" true))))

(event `self.Box.OnComponentBeginOverlap`
  (params (OverlappedComponent :type "PrimitiveComponent Object Reference") (OtherActor :type "Actor Object Reference") (OtherComp :type "PrimitiveComponent Object Reference") (OtherBodyIndex :type Integer) (bFromSweep :type Boolean) (SweepResult :type "HitResult Structure (by ref)"))
  (bind _returnvalue (`self.K2_GetActorLocation`))
  (if (== OtherActor (`GameplayStatics.GetPlayerPawn` 0))
    (bind _returnvalue_2 (`|CreateWidget` "/Game/Blueprints/UI/Text.Text_C"))
    (set `self.Text` _returnvalue_2)
    (`UserWidget.AddToViewport` (`self.Text`) 0)
    (`/Game/Blueprints/UI/Text.UpdateText` (`self.Text`) "Ligma Balls Dom")
    (bind _output_get (set `self.MoveStart` _returnvalue))
    (bind _output_get_2 (set `self.MovEnd` (+ _returnvalue (0.0 -550.0 0.0))))
    (`SkeletalMeshComponent.PlayAnimation` (`self.Mesh`) "/Game/Characters/Animations/AN_Walk_Anim.AN_Walk_Anim" true)
    (`SceneComponent.K2_SetRelativeRotation` (`self.Mesh`) (struct :`Yaw` 90.0) false false)
    (bind (_direction _newtrack_1) (`Timeline|Timeline_0` :!via `PlayFromStart`)
      (:`Update`
        (`self.K2_SetActorLocation` (`KismetMathLibrary.VLerp` _output_get _output_get_2 _newtrack_1))
        (`KismetSystemLibrary.Delay` 3.0)
        (`/Game/Blueprints/UI/Text.UpdateText` (`self.Text`) "")
        (`self.K2_DestroyActor`)))))

(fn `UserConstructionScript`)