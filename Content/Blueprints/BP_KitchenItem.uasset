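; BP_KitchenItem is an interactable kitchen item that receives ingredients for the cooking manager's current recipe.
; On interaction it checks that its name is among the recipe's kitchen items, and prints a refusal message if not.
; Otherwise it stores the ingredient and flags itself cooked once its ingredient count reaches the recipe's, without checking which ingredients were added.
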(event `self.ReceiveBeginPlay`)

(event `/Game/Blueprints/I_InteractInterface.InteractWith`
  (params (CookingManager :type "/Game/Blueprints/BP_CookingManager Object Reference") (Ingredient :type "/Game/Blueprints/BP_Ingredient Object Reference"))
  (bind _currentingredients (`self.CurrentIngredients`))
  (bind (_name _ingredients _mesh _kitchenitems) (break `/Game/Blueprints/BP_RecipeStruct` (`/Game/Blueprints/BP_CookingManager.CurrentRecipe` CookingManager)))
  (if (`KismetArrayLibrary.Array_Contains` _kitchenitems (`self.Name`))
    (`KismetArrayLibrary.Array_Add` _currentingredients Ingredient)
    (if (>= (`KismetArrayLibrary.Array_Length` _currentingredients) (`KismetArrayLibrary.Array_Length` _ingredients))
      (set `self.IsCooked` true)
      (else
        (set `self.IsCooked` false)))
    (else
      (`KismetSystemLibrary.PrintString` "This isn't what I need right now."))))

(fn `UserConstructionScript`)