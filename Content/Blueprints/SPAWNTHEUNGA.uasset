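; Customer spawner actor that places a random customer from ActorList at its Sphere component's transform when SpawnUnga is called.
; It records spawn success in IsSpawned, then runs a cast chain over the six named customer classes to copy that customer's Recipe.
; Most supply Recipe0, while Taro picks randomly from a Recipes array.
; The matched class is removed from ActorList, so it leaves this spawner's pool.
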(event `SpawnUnga`
  (bind _returnvalue (`|SpawnActorFromClass` (`KismetArrayLibrary.Array_Random` (`self.ActorList`)) (`SceneComponent.K2_GetComponentToWorld` (`self.Sphere`)) "Undefined" "OverrideRootScale" null null))
  (set `self.IsSpawned` (`KismetSystemLibrary.IsValid` _returnvalue))
  (bind _asdom_customer (cast `/Game/Blueprints/Customers/Dom_Customer` _returnvalue)
    (:`then`
      (set `self.Recipe` (`/Game/Blueprints/Customers/Dom_Customer.Recipe_0` _asdom_customer))
      (`KismetArrayLibrary.Array_RemoveItem` (`self.ActorList`) (`GameplayStatics.GetObjectClass` _asdom_customer)))
    (:`CastFailed`
      (bind _ascarys_customer (cast `/Game/Blueprints/Customers/Carys_Customer` _returnvalue)
        (:`then`
          (set `self.Recipe` (`/Game/Blueprints/Customers/Carys_Customer.Recipe_0` _ascarys_customer))
          (`KismetArrayLibrary.Array_RemoveItem` (`self.ActorList`) (`GameplayStatics.GetObjectClass` _ascarys_customer)))
        (:`CastFailed`
          (bind _asandre_customer (cast `/Game/Blueprints/Customers/Andre_Customer` _returnvalue)
            (:`then`
              (set `self.Recipe` (`/Game/Blueprints/Customers/Andre_Customer.Recipe_0` _asandre_customer))
              (`KismetArrayLibrary.Array_RemoveItem` (`self.ActorList`) (`GameplayStatics.GetObjectClass` _asandre_customer)))
            (:`CastFailed`
              (bind _asdan_customer (cast `/Game/Blueprints/Customers/Dan_Customer` _returnvalue)
                (:`then`
                  (set `self.Recipe` (`/Game/Blueprints/Customers/Dan_Customer.Recipe_0` _asdan_customer))
                  (`KismetArrayLibrary.Array_RemoveItem` (`self.ActorList`) (`GameplayStatics.GetObjectClass` _asdan_customer)))
                (:`CastFailed`
                  (bind _assteph_customer (cast `/Game/Blueprints/Customers/Steph_Customer` _returnvalue)
                    (:`then`
                      (set `self.Recipe` (`/Game/Blueprints/Customers/Steph_Customer.Recipe_0` _assteph_customer))
                      (`KismetArrayLibrary.Array_RemoveItem` (`self.ActorList`) (`GameplayStatics.GetObjectClass` _assteph_customer)))
                    (:`CastFailed`
                      (bind _astaro_customer (cast `/Game/Blueprints/Customers/Taro_Customer` _returnvalue))
                      (bind _recipes (`/Game/Blueprints/Customers/Taro_Customer.Recipes` _astaro_customer))
                      (set `self.Recipe` (`|GetArrayItem` _recipes (`KismetMathLibrary.RandomInteger` (`KismetArrayLibrary.Array_Length` _recipes))))
                      (`KismetArrayLibrary.Array_RemoveItem` (`self.ActorList`) (`GameplayStatics.GetObjectClass` _astaro_customer)))))))))))))

(fn `UserConstructionScript`)