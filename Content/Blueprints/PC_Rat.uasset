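; Player rat character that walks, yaw-turns with turn-direction flags, and picks up ingredients in a cooking game.
; On BeginPlay it finds or spawns the BP_CookingManager.
; Interact sphere-traces for a BP_IngredientSpawn, notifies it, then spawns its ingredient and attaches it to HandSocket after a short delay.
; A drop branch and Tick physics-handle update depend on IsGrabbingObject, which only disconnected line-trace grab leftovers set true.
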(event `InputAxis|Input_Walk`
  (params (AxisValue :type "Float (single-precision)"))
  (`self.AddMovementInput` (`self.GetActorForwardVector`) AxisValue))

(event `InputAxis|Input_LeftRight`
  (params (AxisValue :type "Float (single-precision)"))
  (bind _returnvalue (`self.GetInputAxisValue`))
  (`self.AddControllerYawInput` AxisValue)
  (if true
    (`|ExecutionSequence`
      (:`then_0`
        (if (> _returnvalue 0.3)
          (`self.TurnRight/Left?` true)
          (else
            (set `self.TurnRight` false))))
      (:`then_1`
        (if (< _returnvalue -0.3)
          (`self.TurnRight/Left?` false true)
          (else
            (set `self.TurnLeft` false)))))))

(event `self.ReceiveBeginPlay`
  (bind _returnvalue (`GameplayStatics.GetActorOfClass` "/Game/Blueprints/BP_CookingManager.BP_CookingManager_C"))
  (if (`KismetSystemLibrary.IsValid` _returnvalue)
    (set `self.CookingMngr` _returnvalue)
    (else
      (bind _returnvalue_2 (`|SpawnActorFromClass` "/Game/Blueprints/BP_CookingManager.BP_CookingManager_C" (`self.GetTransform`) "Undefined" "OverrideRootScale" null null))
      (set `self.CookingMngr` _returnvalue_2))))

(event `InputAction|Interact`
  (params (Key :type "Key Structure"))
  (bind _capsulecomponent (`self.CapsuleComponent`))
  (bind _heldingredient (`self.HeldIngredient`))
  (bind _mesh (`self.Mesh`))
  (bind _handsocket (`self.HandSocket`))
  (bind _returnvalue (`SceneComponent.K2_GetComponentLocation` _capsulecomponent))
  (:`Pressed`
    (if (`self.IsGrabbingObject `)
      (`SceneComponent.K2_DetachFromComponent` (`StaticMeshActor.StaticMeshComponent` _heldingredient) "KeepRelative" "KeepRelative" "KeepRelative" true)
      (`PrimitiveComponent.SetSimulatePhysics` (`StaticMeshActor.StaticMeshComponent` _heldingredient) true)
      (set `self.IsGrabbingObject ` false)
      (else
        (bind _outhit (`KismetSystemLibrary.SphereTraceSingle` _returnvalue (+ _returnvalue (* (`KismetMathLibrary.GetForwardVector` (`SceneComponent.K2_GetComponentRotation` _capsulecomponent)) (`self.InteractRange`))) 30.0 "TraceTypeQuery3"))
        (bind _asbp_ingredient_spawn (cast `/Game/Blueprints/BP_IngredientSpawn` (`.HitActor` (`GameplayStatics.BreakHitResult` _outhit))))
        (message `/Game/Blueprints/I_InteractInterface.InteractWith` _asbp_ingredient_spawn (`self.CookingMngr`))
        (bind _returnvalue_2 (`|SpawnActorFromClass` "/Game/Blueprints/BP_Ingredient.BP_Ingredient_C" (`SceneComponent.GetSocketTransform` _mesh _handsocket "RTS_World") "Undefined" "OverrideRootScale" null (`/Game/Blueprints/BP_IngredientSpawn.SpawnIngredient` _asbp_ingredient_spawn) null))
        (bind _output_get (set `self.HeldIngredient` _returnvalue_2))
        (`KismetSystemLibrary.Delay` 0.2)
        (`self.K2_AttachToComponent` _output_get _mesh _handsocket "SnapToTarget" "SnapToTarget" "SnapToTarget" true)))))

(event `self.ReceiveTick`
  (params (DeltaSeconds :type "Float (single-precision)"))
  (bind _hold_place (`self.Hold Place`))
  (if (`self.IsGrabbingObject `)
    (`PhysicsHandleComponent.SetTargetLocation` (`self.PhysicsHandle`) (+ (`SceneComponent.K2_GetComponentLocation` _hold_place) (* (`KismetMathLibrary.GetForwardVector` (`SceneComponent.K2_GetComponentRotation` _hold_place)) 50.0)))))

(fn `UserConstructionScript`)