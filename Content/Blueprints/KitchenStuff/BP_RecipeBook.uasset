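; BP_RecipeBook is an interactable kitchen recipe book that shows an on-screen recipe UI.
; On BeginPlay it creates the RecipeBook widget, adds it to the viewport and hides it.
; Interactwith makes the widget visible, then flags the book as open on the CookingManager and hands it the widget reference.
; A disconnected, never-run chain would set text from the Customer_Generic's current recipe row.
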(event `self.ReceiveBeginPlay`
  (bind _returnvalue (`|CreateWidget` "/Game/Blueprints/UI/RecipeBook.RecipeBook_C"))
  (bind _output_get (set `self.UI_RecipeBook` _returnvalue))
  (`UserWidget.AddToViewport` _returnvalue 0)
  (`Widget.SetVisibility` _output_get "Hidden")
  (set `self.IsOpen` false))

(event `/Game/Blueprints/KitchenStuff/I_InteractInterface.InteractWith`
  (params (CookingManager :type "/Game/Blueprints/KitchenStuff/BP_CookingManager Object Reference") (Ingredient :type "/Game/Blueprints/KitchenStuff/BP_Ingredient Object Reference"))
  (`Widget.SetVisibility` (`self.UI_RecipeBook`) "Visible")
  (set `/Game/Blueprints/KitchenStuff/BP_CookingManager.BookIsOpen` true CookingManager)
  (set `/Game/Blueprints/KitchenStuff/BP_CookingManager.UIRecipeBook` (`self.UI_RecipeBook`) CookingManager))

(fn `UserConstructionScript`)