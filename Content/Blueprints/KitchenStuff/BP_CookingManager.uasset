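; Cooking manager that runs the customer order loop in the kitchen, tracking the current recipe and its needed ingredients.
; On BeginPlay it finds or spawns the customer spawner, spawns a customer and loads that customer's recipe from its data table row.
; A speech bubble widget shows the order, name and image briefly, using fixed delays to match walk-in time.
; FoodCooked removes the current recipe, then brings in the next customer.
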(event `self.ReceiveBeginPlay`
  (bind _speechbubble (`self.SpeechBubble`))
  (bind _customerspawner (`self.CustomerSpawner`))
  (bind _returnvalue (`GameplayStatics.GetActorOfClass` "/Game/Blueprints/SPAWNTHEUNGA.SPAWNTHEUNGA_C"))
  (bind _output_get (set `self.CustomerSpawner` _returnvalue))
  (`/Engine/EditorBlueprintResources/StandardMacros.IsValid` _output_get
    (:`Is Valid`
      _)
    (:`Is Not Valid`
      (bind _returnvalue_2 (`|SpawnActorFromClass` "/Game/Blueprints/SPAWNTHEUNGA.SPAWNTHEUNGA_C" (`self.GetTransform`) "Undefined" "OverrideRootScale" null null))
      (set `self.CustomerSpawner` _returnvalue_2)))
  (if (`KismetArrayLibrary.Array_IsNotEmpty` (`self.Recipes`))
    ;[1 1 1] Makes speech bubble UI canvas, but hides it until customer sits
    (bind _returnvalue_3 (`|CreateWidget` "/Game/Blueprints/UI/SpeechBubble.SpeechBubble_C"))
    (bind _output_get_2 (set `self.SpeechBubble` _returnvalue_3))
    (`UserWidget.AddToViewport` _output_get_2 0)
    (`Widget.SetVisibility` (`self.SpeechBubble`) "Hidden")
    (`/Game/Blueprints/SPAWNTHEUNGA.SpawnUnga` _customerspawner)
    (`self.GetNewRecipe` (`/Game/Blueprints/SPAWNTHEUNGA.Recipe` _customerspawner))
    (`KismetSystemLibrary.Delay` 3.0)
    (`Widget.SetVisibility` _speechbubble "Visible") ; Turns on speech bubble UI when customer sits (delay value is time taken for customer to walk to table)
    (`KismetSystemLibrary.Delay` 3.0)
    (`Widget.SetVisibility` _speechbubble "Hidden") ; Turns off speech bubble after 3 seconds
  ))

(event `FoodCooked`
  (bind _speechbubble (`self.SpeechBubble`))
  (bind _customerspawner (`self.CustomerSpawner`))
  (`KismetArrayLibrary.Array_Remove` (`self.Recipes`) (`self.CurrentRecipeIndex`))
  (`KismetSystemLibrary.Delay` 3.0) ; delay between serving customer and next one coming in
  (`/Game/Blueprints/SPAWNTHEUNGA.SpawnUnga` _customerspawner)
  (`self.GetNewRecipe` (`/Game/Blueprints/SPAWNTHEUNGA.Recipe` _customerspawner))
  ;[1 1 1] Makes canvas visible for three seconds when customer requests dish, then turns it off (again!)
  (`KismetSystemLibrary.Delay` 3.0) ; time taken for new customer to walk in
  (`Widget.SetVisibility` _speechbubble "Visible")
  (`KismetSystemLibrary.Delay` 3.0)
  (`Widget.SetVisibility` _speechbubble "Hidden"))

(fn `GetNewRecipe`
  (params (Recipe :type "DataTableRowHandle Structure"))
  (returns (RecipeText :type "/Game/Blueprints/UI/SpeechBubble Object Reference"))
  (bind (_datatable _rowname) (break `DataTableRowHandle` Recipe))
  (bind _speechbubble (`self.SpeechBubble`))
  (bind ((`CustomerName_24_220C5CFE4DF498D791DFC68636715360` _customername) (`CustomerImage_30_AA593C8F422C4BAA9A0E608C1CBF85DA` _customerimage)) (break `/Game/Blueprints/KitchenStuff/BP_RecipeStruct` (`self.CurrentRecipe`)))
  (`/Engine/EditorBlueprintResources/StandardMacros.IsValid` _datatable
    (:`Is Valid`
      (bind _returnvalue (`|GetDataTableRow` _datatable _rowname)
        (:`then`
          (bind _output_get (set `self.CurrentRecipe` _returnvalue))
          (set `self.CurrentRecipeIndex` (`KismetArrayLibrary.Array_Find` (`self.Recipes`) Recipe))
          (set `self.NeededIngredients` (`.Ingredients_16_69F9478048B65A31BBCA62AC47C03B29` (break `/Game/Blueprints/KitchenStuff/BP_RecipeStruct` _output_get)))
          ;[1 1 1] Update Customer UI
          (`/Game/Blueprints/UI/SpeechBubble.UpdateText` _speechbubble (`KismetTextLibrary.Conv_NameToText` _rowname)) ; WHAT RECIPE THEY SAY
          (`/Game/Blueprints/UI/SpeechBubble.UpdateName` _speechbubble _customername)
          (`/Game/Blueprints/UI/SpeechBubble.UpdateImage` _speechbubble _customerimage)
          (return (`self.SpeechBubble`)))))))

(fn `UserConstructionScript`)