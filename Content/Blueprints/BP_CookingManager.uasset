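; Cooking manager actor that sets the current dish order and judges cooked food against it.
; On BeginPlay it finds or spawns the SPAWNTHEUNGA customer spawner and, if recipes remain, spawns a customer whose recipe GetNewRecipe reads from a data table and shows in a text widget, cleared after a delay.
; FoodCooked removes a matching recipe and calls GetNewRecipe again with no recipe supplied, or prints a wrong-dish message.
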(event `self.ReceiveBeginPlay`
  (bind _customerspawner (`self.CustomerSpawner`))
  (bind _returnvalue (`GameplayStatics.GetActorOfClass` "/Game/Blueprints/SPAWNTHEUNGA.SPAWNTHEUNGA_C"))
  (bind _output_get (set `self.CustomerSpawner` _returnvalue))
  (`/Engine/EditorBlueprintResources/StandardMacros.IsValid` _output_get
    (:`Is Valid`
      _)
    (:`Is Not Valid`
      (bind _returnvalue_2 (`|SpawnActorFromClass` "/Game/Blueprints/SPAWNTHEUNGA.SPAWNTHEUNGA_C" (`self.GetTransform`) "Undefined" "OverrideRootScale" null null))
      (set `self.CustomerSpawner` _returnvalue_2)))
  (if (`KismetArrayLibrary.Array_IsNotEmpty` (`self.Recipes`))
    (`/Game/Blueprints/SPAWNTHEUNGA.SpawnUnga` _customerspawner)
    (bind _recipetext (`self.GetNewRecipe` (`/Game/Blueprints/SPAWNTHEUNGA.Recipe` _customerspawner)))
    (`KismetSystemLibrary.Delay` 3.0)
    (`/Game/Blueprints/UI/Text.UpdateText` _recipetext " ")))

(event `FoodCooked`
  (params (DishName :type String))
  (if (`KismetStringLibrary.EqualEqual_StrStr` DishName (`.Name_14_DE6BDE0C4E226A4E7091B69701C4008F` (break `/Game/Blueprints/BP_RecipeStruct` (`self.CurrentRecipe`))))
    (`KismetArrayLibrary.Array_Remove` (`self.Recipes`) (`self.CurrentRecipeIndex`))
    (bind _recipetext (`self.GetNewRecipe` (struct)))
    (`KismetSystemLibrary.Delay` 3.0)
    (`/Game/Blueprints/UI/Text.UpdateText` _recipetext " ")
    (else
      (`KismetSystemLibrary.PrintString` "Cringe, that's the wrong dish nerd!"))))

(fn `GetNewRecipe`
  (params (Recipe :type "DataTableRowHandle Structure"))
  (returns (RecipeText :type "/Game/Blueprints/UI/Text Object Reference"))
  (bind (_datatable _rowname) (break `DataTableRowHandle` Recipe))
  (`/Engine/EditorBlueprintResources/StandardMacros.IsValid` _datatable
    (:`Is Valid`
      (bind _returnvalue (`|GetDataTableRow` _datatable _rowname)
        (:`then`
          (set `self.CurrentRecipe` _returnvalue)
          (set `self.CurrentRecipeIndex` (`KismetArrayLibrary.Array_Find` (`self.Recipes`) Recipe))
          (bind _returnvalue_2 (`|CreateWidget` "/Game/Blueprints/UI/Text.Text_C"))
          (bind _output_get (set `self.RecipeText` _returnvalue_2))
          (`UserWidget.AddToViewport` _output_get 0)
          (`/Game/Blueprints/UI/Text.UpdateText` (`self.RecipeText`) (`KismetTextLibrary.Conv_NameToText` _rowname))
          (return (`self.RecipeText`)))))))

(fn `UserConstructionScript`)